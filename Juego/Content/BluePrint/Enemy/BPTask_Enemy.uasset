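; BPTask_Enemy is a Behavior Tree task that picks the next patrol point for a BP_enemyCharacter.
; It writes the location of the current TargetPoint array entry to the BBLoc blackboard key, then advances its Index, resetting it to zero after the last entry.
; FinishExecute runs only on the increment branch, so the task does not finish when the index wraps or the cast fails.
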(event `self.ReceiveExecuteAI`
  (params (OwnerController :type "AIController Object Reference") (ControlledPawn :type "Pawn Object Reference"))
  (bind _asbp_enemy_character (cast `/Game/BluePrint/Enemy/BP_enemyCharacter` ControlledPawn))
  (bind _targetpoint (`/Game/BluePrint/Enemy/BP_enemyCharacter.TargetPoint` _asbp_enemy_character))
  (`BTFunctionLibrary.SetBlackboardValueAsVector` (`self.BBLoc`) (`Actor.K2_GetActorLocation` (`|GetArrayItem` _targetpoint (`self.index`))))
  (if (>= (`self.index`) (- (`KismetArrayLibrary.Array_Length` _targetpoint) 1))
    (set `self.index` 0)
    (else
      (`/Engine/EditorBlueprintResources/StandardMacros.IncrementInt` (`self.index`)
        (:`  `
          (`self.FinishExecute` true))))))